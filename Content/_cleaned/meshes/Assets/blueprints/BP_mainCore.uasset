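; BP_mainCore is an actor with two door meshes that swing open when an actor overlaps it and close after a short delay once overlap ends.
; The Construction Script caches each door's initial relative rotation.
; A single timeline, DoorA_slide, adds the same yaw offset to both cached rotations, so despite its name the doors rotate rather than slide.
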(event EventActorBeginOverlap
  (params (OtherActor :type Actor%20Object%20Reference))
  (bind _doora_initialrotation (Variables|Default|GetdoorA_initialRotation))
  (bind _doorb_initialrotation (Variables|Default|GetdoorB_initialRotation))
  (bind (_pitch _yaw _roll) (Class|KismetMathLibrary|BreakRot _doorb_initialrotation))
  (bind (_pitch_2 _yaw_2 _roll_2) (Class|KismetMathLibrary|BreakRot _doora_initialrotation))
  (bind _z_rotation_ (Timeline|doorA_slide Play)
    (:Update
      (Transformation|SetRelativeRotation (Variables|Default|GetdoorA) (Class|KismetMathLibrary|MakeRot _pitch_2 (+ _z_rotation_ _yaw_2) _roll_2) false)
      (Transformation|SetRelativeRotation (Variables|Default|GetdoorB) (Class|KismetMathLibrary|MakeRot _pitch (+ _z_rotation_ _yaw) _roll) false))))

(event EventActorEndOverlap
  (params (OtherActor :type Actor%20Object%20Reference))
  (bind _doora_initialrotation (Variables|Default|GetdoorA_initialRotation))
  (bind _doorb_initialrotation (Variables|Default|GetdoorB_initialRotation))
  (bind (_pitch _yaw _roll) (Class|KismetMathLibrary|BreakRot _doorb_initialrotation))
  (bind (_pitch_2 _yaw_2 _roll_2) (Class|KismetMathLibrary|BreakRot _doora_initialrotation))
  (Utilities|FlowControl|Delay 1.5)
  (bind _z_rotation_ (Timeline|doorA_slide Reverse)
    (:Update
      (Transformation|SetRelativeRotation (Variables|Default|GetdoorA) (Class|KismetMathLibrary|MakeRot _pitch_2 (+ _z_rotation_ _yaw_2) _roll_2) false)
      (Transformation|SetRelativeRotation (Variables|Default|GetdoorB) (Class|KismetMathLibrary|MakeRot _pitch (+ _z_rotation_ _yaw) _roll) false))))

(fn ConstructionScript
  (Variables|Default|SetdoorA_initialRotation (Variables|/Script/Engine.SceneComponent|GetRelativeRotation (Variables|Default|GetdoorA)))
  (Variables|Default|SetdoorB_initialRotation (Variables|/Script/Engine.SceneComponent|GetRelativeRotation (Variables|Default|GetdoorB))))