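; Game mode for a Brainzlab match that spawns up to four professor characters, human or AI, and shows a timer.
; Construction derives the AI count from the game instance's player slots and picks the first player's male or female pawn class.
; BeginPlay creates the other local players, switching pawn class before each, and spawns AI professors with assigned materials.
; Escape or the LoadCredits flag cleans up and returns to the menu level.
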(event EventBeginPlay
  (bind _returnvalue (UserInterface|CreateWidget "/Game/Blueprints/UI/TimerWidgetBP.TimerWidgetBP_C"))
  (Variables|Default|SetTimerWidget _returnvalue)
  (UserInterface|Viewport|AddtoViewport (Variables|Default|GetTimerWidget))
  (bind _asbrainzlapgameinstance (Utilities|Casting|CastToBrainzlapGameInstance (Game|GetGameInstance)))
  (Variables|/Script/CapTheBrain.TimerWidget|SettotalMinutes _returnvalue (Variables|/Script/CapTheBrain.BrainzlapGameInstance|Getminutes _asbrainzlapgameinstance))
  (Variables|/Script/CapTheBrain.TimerWidget|SetminutesLeft _returnvalue (Variables|/Script/CapTheBrain.BrainzlapGameInstance|Getminutes _asbrainzlapgameinstance))
  (for _index (range 1 (- (Variables|/Script/CapTheBrain.BrainzlapGameInstance|GetplayerCount _asbrainzlapgameinstance) 1))
    (if (Utilities|Array|Get(acopy) (Variables|/Script/CapTheBrain.BrainzlapGameInstance|GetmaleChar _asbrainzlapgameinstance) _index)
      (Variables|Default|SetDefaultPawnClass "/Game/Blueprints/Characters/Professor.Professor_C")
      (else
        (Variables|Default|SetDefaultPawnClass "/Game/Blueprints/Characters/Professorin.Professorin_C")))
    (bind _returnvalue_2 (Class|GameplayStatics|CreatePlayer 0 _index))
    (Class|CaptheBrainArenaGameMode|SetPlayerMaterial (Pawn|GetControlledPawn _returnvalue_2) (Utilities|Array|Get(acopy) (Variables|/Script/CapTheBrain.BrainzlapGameInstance|GetplayerMats _asbrainzlapgameinstance) _index)))
  (for _index_2 (range 0 (- (Variables|Default|GetKICount) 1))
    (bind _returnvalue_3 (Game|SpawnActorfromClass "/Game/Blueprints/Characters/AI/ProfAI.ProfAI_C" (Math|Conversions|ToTransform(Vector) "1799.000000,1923.000488,100.000000") true 0))
    (Pawn|SpawnDefaultController _returnvalue_3)
    (Class|CaptheBrainCharacter|SetMaterial _returnvalue_3 (Utilities|Array|Get(acopy) (Variables|/Script/CapTheBrain.BrainzlapGameInstance|GetKIMats _asbrainzlapgameinstance) _index_2)))
  (Variables|Default|Setstarting true))

(event EventTick
  (params (DeltaSeconds :type Float%20%28single-precision%29))
  (bind _asbrainzlapgameinstance (Utilities|Casting|CastToBrainzlapGameInstance (Game|GetGameInstance)))
  (if (Variables|/Script/CapTheBrain.BrainzlapGameInstance|GetloadCredits _asbrainzlapgameinstance)
    (Class|UserWidget|RemovefromViewport (Variables|Default|GetTimerWidget))
    (Class|BrainzlapGameInstance|CleanUp _asbrainzlapgameinstance)
    (Variables|/Script/CapTheBrain.BrainzlapGameInstance|Setrestart _asbrainzlapgameinstance true)
    (Game|OpenLevel(byName) 0 "BrainzlabMenu" true "?game=/Game/Blueprints/MenuGameModeBP.MenuGameModeBP")))

(event Input|KeyboardEvents|Escape
  (:Pressed
    (Class|UserWidget|RemovefromViewport (Variables|Default|GetTimerWidget))
    (Class|BrainzlapGameInstance|CleanUp (stale EventTick _asbrainzlapgameinstance))
    (Variables|/Script/CapTheBrain.BrainzlapGameInstance|Setrestart (stale EventTick _asbrainzlapgameinstance) true)
    (Game|OpenLevel(byName) 0 "BrainzlabMenu" true "?game=/Game/Blueprints/MenuGameModeBP.MenuGameModeBP")))

(fn ConstructionScript
  (bind _asbrainzlapgameinstance (Utilities|Casting|CastToBrainzlapGameInstance (Game|GetGameInstance)))
  (Variables|Default|SetKICount (- 4 (Utilities|Array|Length (Variables|/Script/CapTheBrain.BrainzlapGameInstance|GetmaleChar _asbrainzlapgameinstance))))
  (if (Utilities|Array|Get(acopy) (Variables|/Script/CapTheBrain.BrainzlapGameInstance|GetmaleChar _asbrainzlapgameinstance))
    (Variables|Default|SetDefaultPawnClass "/Game/Blueprints/Characters/Professor.Professor_C")
    (else
      (Variables|Default|SetDefaultPawnClass "/Game/Blueprints/Characters/Professorin.Professorin_C"))))