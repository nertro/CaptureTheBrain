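; Game mode for the Brainzlab credits screen, which shows a UI widget and handles the return to the main menu.
; On BeginPlay it shows the mouse cursor and adds an ExploreWidget, stored as CreditsWidget, to the viewport.
; LoadMenu removes that widget, cleans up the game instance, flags WasInExplore, and opens the menu level with the menu game mode passed as a URL option.
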(event EventBeginPlay
  (Variables|/Script/Engine.PlayerController|SetbShowMouseCursor (Game|GetPlayerController 0) true)
  (bind _returnvalue (UserInterface|CreateWidget "/Game/Credits/ExploreWidget.ExploreWidget_C"))
  (Variables|Default|SetCreditsWidget _returnvalue)
  (UserInterface|Viewport|AddtoViewport (Variables|Default|GetCreditsWidget)))

(fn ConstructionScript)

(fn LoadMenu
  (Class|UserWidget|RemovefromViewport (Variables|Default|GetCreditsWidget))
  (bind _asbrainzlapgameinstance (Utilities|Casting|CastToBrainzlapGameInstance (Game|GetGameInstance)))
  (Class|BrainzlapGameInstance|CleanUp _asbrainzlapgameinstance)
  (Variables|/Script/CapTheBrain.BrainzlapGameInstance|SetwasInExplore _asbrainzlapgameinstance true)
  (Game|OpenLevel(byName) "BrainzlabMenu" true "?game=/Game/Blueprints/MenuGameModeBP.MenuGameModeBP"))