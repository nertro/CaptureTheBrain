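; Menu game mode for Brainzlap that creates the menu-flow widgets, plays the intro or restart credits, and opens the game and explore levels.
; BeginPlay disables player controllers, finds ambient sounds by display name, then calls StartNewGame after game over or plays the unseen intro.
; Tick polls intro and credits audio to detect their end, then shows the menu, spawns the brain and starts background sound.
; Game instance flags carry state, and level loads override the game mode through options.
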(event EventBeginPlay
  (bind _introplayer (Variables|Default|GetintroPlayer))
  (bind _outactors (Actor|GetAllActorsOfClass "/Script/Engine.PlayerController"))
  (for _array_element _outactors
    (bind _asplayercontroller (Utilities|Casting|CastToPlayerController _array_element))
    (Class|BrainzlabMenuGameMode|DisableController _asplayercontroller))
  (bind _asbrainzlapgameinstance (Utilities|Casting|CastToBrainzlapGameInstance (Game|GetGameInstance)))
  (Variables|/Script/Engine.PlayerController|SetbShowMouseCursor (Game|GetPlayerController 0) true)
  (Variables|Default|SetTempProfMats (Variables|Default|GetprofMats))
  (Variables|Default|SetTempProfInMats (Variables|Default|GetprofInMats))
  (bind _returnvalue (UserInterface|CreateWidget "/Game/Menu/MenuWidget.MenuWidget_C"))
  (Variables|Default|SetMenuWidget _returnvalue)
  (bind _returnvalue_2 (UserInterface|CreateWidget "/Game/Menu/ControlsWidget.ControlsWidget_C"))
  (Variables|Default|SetControlsWidget _returnvalue_2)
  (bind _returnvalue_3 (UserInterface|CreateWidget "/Game/Menu/ItemExplWidget.ItemExplWidget_C"))
  (Variables|Default|SetItemWidget _returnvalue_3)
  (bind _returnvalue_4 (UserInterface|CreateWidget "/Game/Menu/IntroWidget.IntroWidget_C"))
  (Variables|Default|SetIntroWidget _returnvalue_4)
  (bind _returnvalue_5 (UserInterface|CreateWidget "/Game/Menu/CreditsWidget.CreditsWidget_C"))
  (Variables|Default|SetCreditsWidget _returnvalue_5)
  (bind _returnvalue_6 (UserInterface|CreateWidget "/Game/Menu/ArrowsWidget.ArrowsWidget_C"))
  (Variables|Default|SetArrowsWidget _returnvalue_6)
  (bind _returnvalue_7 (UserInterface|CreateWidget "/Game/Menu/TutorialWidget.TutorialWidget_C"))
  (Variables|Default|SetTutorialWidget _returnvalue_7)
  (bind _returnvalue_8 (UserInterface|CreateWidget "/Game/Menu/PlayerCountWidget.PlayerCountWidget_C"))
  (Variables|Default|SetPlayerCountWidget _returnvalue_8)
  (bind _returnvalue_9 (UserInterface|CreateWidget "/Game/Menu/PlayerSelectWidget.PlayerSelectWidget_C"))
  (Variables|Default|SetPlayerSelectWidget _returnvalue_9)
  (bind _returnvalue_10 (UserInterface|CreateWidget "/Game/Menu/SetTimeWidget.SetTimeWidget_C"))
  (Variables|Default|SetSetTimeWidget _returnvalue_10)
  (CallFunction|GetSounds)
  (if (Variables|/Script/CapTheBrain.BrainzlapGameInstance|GetgameOver _asbrainzlapgameinstance)
    (Class|BrainzlabMenuGameMode|StartNewGame)
    (elif (not (Variables|/Script/CapTheBrain.BrainzlapGameInstance|GetintroPlayed _asbrainzlapgameinstance))
      (UserInterface|Viewport|AddtoViewport (Variables|Default|GetIntroWidget))
      (Audio|Components|Audio|Play (Variables|Default|GetIntroSound) 0.0)
      (Class|MediaPlayer|Rewind _introplayer)
      (Media|MediaPlayer|Play _introplayer :!class /Script/MediaAssets.MediaPlayer)
      (Variables|Default|SetintroIsPlaying true))))

(event EventTick
  (params (DeltaSeconds :type Float%20%28single-precision%29))
  (bind _creditsplayer (Variables|Default|GetcreditsPlayer))
  (bind _asbrainzlapgameinstance (Utilities|Casting|CastToBrainzlapGameInstance (Game|GetGameInstance)))
  (if (Variables|/Script/CapTheBrain.BrainzlapGameInstance|Getrestart _asbrainzlapgameinstance)
    (UserInterface|Viewport|AddtoViewport (Variables|Default|GetCreditsWidget))
    (Audio|Components|Audio|Play (Variables|Default|GetCreditsSound) 0.0)
    (Class|MediaPlayer|Rewind _creditsplayer)
    (Media|MediaPlayer|Play _creditsplayer :!class /Script/MediaAssets.MediaPlayer)
    (Variables|Default|SetcreditsIsPlaying true)
    (Variables|/Script/CapTheBrain.BrainzlapGameInstance|Setrestart _asbrainzlapgameinstance false)
    (else
      (bind _returnvalue (Audio|Components|Audio|IsPlaying (Variables|Default|GetIntroSound)))
      (bind _returnvalue_2 (Audio|Components|Audio|IsPlaying (Variables|Default|GetCreditsSound)))
      (if (Variables|Default|GetintroIsPlaying)
        (if (not _returnvalue)
          (CallFunction|ChangeWidget (Variables|Default|GetMenuWidget) (Variables|Default|GetIntroWidget))
          (Variables|Default|SetintroIsPlaying false)
          (Variables|/Script/CapTheBrain.BrainzlapGameInstance|SetintroPlayed _asbrainzlapgameinstance true)
          (CallFunction|SpawnBrain :!label _label)
          (Audio|Components|Audio|Play (Variables|Default|GetBackGroundSound) 0.0))
        (elif (Variables|Default|GetcreditsIsPlaying)
          (if (not _returnvalue_2)
            (CallFunction|ChangeWidget (Variables|Default|GetMenuWidget) (Variables|Default|GetCreditsWidget))
            (Variables|Default|SetcreditsIsPlaying false)
            (Class|BrainzlapGameInstance|RestartGame _asbrainzlapgameinstance)
            (goto _label)))))))

(fn ConstructionScript)

(fn LoadExplore
  (Class|UserWidget|RemovefromViewport (Variables|Default|GetMenuWidget))
  (bind _asbrainzlapgameinstance (Utilities|Casting|CastToBrainzlapGameInstance (Game|GetGameInstance)))
  (Variables|/Script/CapTheBrain.BrainzlapGameInstance|SetcurCharacter _asbrainzlapgameinstance 0)
  (Game|OpenLevel(byName) "BrainzlabExplore" true "?game=/Game/Blueprints/BrainzlabCreditsGameModeBP.BrainzlabCreditsGameModeBP"))

(fn LoadGame
  (Variables|/Script/Engine.PlayerController|SetbShowMouseCursor (Game|GetPlayerController 0) false)
  (Class|UserWidget|RemovefromViewport (Variables|Default|GetPlayerCountWidget))
  (bind _asbrainzlapgameinstance (Utilities|Casting|CastToBrainzlapGameInstance (Game|GetGameInstance)))
  (Variables|/Script/CapTheBrain.BrainzlapGameInstance|SetcurCharacter _asbrainzlapgameinstance 0)
  (Variables|/Script/CapTheBrain.BrainzlapGameInstance|SetgameStarted _asbrainzlapgameinstance true)
  (Game|OpenLevel(byName) "CapTheBrain_Level" false "?game=/Game/Blueprints/BrainzlabGameMode.BrainzlabGameMode"))

(fn SpawnBrain
  (bind _asbrainzlapgameinstance (Utilities|Casting|CastToBrainzlapGameInstance (Game|GetGameInstance)))
  (bind _returnvalue (Game|SpawnActorfromClass "/Game/Blueprints/Items/BrainBlueprint.BrainBlueprint_C" (Math|Transform|MakeTransform (Variables|Default|GetBrainPos) "0,180.000000, 0" "1.000000,1.000000,1.000000") true 0))
  (Variables|/Script/CapTheBrain.BrainzlapGameInstance|SetcurCharacter _asbrainzlapgameinstance _returnvalue)
  (Audio|Components|Audio|Play (Variables|Default|GetBrainSound) 0.0))

(fn ChangeWidget
  (params (newWidget :type User%20Widget%20Object%20Reference) (oldWidget :type User%20Widget%20Object%20Reference))
  (UserInterface|Viewport|AddtoViewport newWidget)
  (Class|UserWidget|RemovefromViewport oldWidget))

(fn GetSounds
  (bind _outactors (Actor|GetAllActorsOfClass "/Script/Engine.AmbientSound"))
  (for _array_element _outactors
    (if (Utilities|Enum|Equal(Enum) (Utilities|GetDisplayName _array_element) "BrainSound")
      (bind _asambientsound (Utilities|Casting|CastToAmbientSound _array_element))
      (Variables|Default|SetBrainSound _asambientsound)
      (elif (Utilities|Enum|Equal(Enum) (Utilities|GetDisplayName _array_element) "BackgrSound")
        (bind _asambientsound_2 (Utilities|Casting|CastToAmbientSound _array_element))
        (Variables|Default|SetBackGroundSound _asambientsound_2)
        (elif (Utilities|Enum|Equal(Enum) (Utilities|GetDisplayName _array_element) "IntroSound")
          (bind _asambientsound_3 (Utilities|Casting|CastToAmbientSound _array_element))
          (Variables|Default|SetIntroSound _asambientsound_3)
          (elif (Utilities|Enum|Equal(Enum) (Utilities|GetDisplayName _array_element) "CreditsSound")
            (bind _asambientsound_4 (Utilities|Casting|CastToAmbientSound _array_element))
            (Variables|Default|SetCreditsSound _asambientsound_4)))))))