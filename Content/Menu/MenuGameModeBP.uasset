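; Game mode for the main menu that shows the menu UI and launches levels.
; On BeginPlay it enables the mouse cursor, creates the menu and controls widgets, and adds only the menu to the viewport.
; LoadGame removes the menu widget and opens the level given by name with the supplied options.
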(event EventBeginPlay
  (Variables|/Script/Engine.PlayerController|SetbShowMouseCursor (Game|GetPlayerController 0) true)
  (bind _returnvalue (UserInterface|CreateWidget "/Game/Menu/MenuWidget.MenuWidget_C"))
  (Variables|Default|SetMenuWidget _returnvalue)
  (bind _returnvalue_2 (UserInterface|CreateWidget "/Game/Menu/ControlsWidget.ControlsWidget_C"))
  (Variables|Default|SetControlsWidget _returnvalue_2)
  (UserInterface|Viewport|AddtoViewport (Variables|Default|GetMenuWidget)))

(fn ConstructionScript)

(fn LoadGame
  (params (LevelName :type Name :default "None") (LevelOptions :type String))
  (Class|UserWidget|RemovefromViewport (Variables|Default|GetMenuWidget))
  (Game|OpenLevel(byName) LevelName true LevelOptions))